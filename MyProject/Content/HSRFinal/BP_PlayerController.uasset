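; BP_PlayerController creates the player's party of four role-based characters: single-target DPS, AOE DPS, buffer and sustain.
; On BeginPlay it spawns one of each at its own transform and stores them as Player1 through Player4.
; It then hides all four in game, with no logic here to show, switch or control them.
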(event EventBeginPlay
  ;[0.15 0.15 0.15 0.5] set reference to each individual player character
  (bind _returnvalue (Game|SpawnActorfromClass "/Game/HSRFinal/TBPlayer/Player/BP_STDPS.BP_STDPS_C" (Transformation|GetActorTransform) "Undefined" "MultiplyWithRoot" 0 0))
  (Variables|Default|SetPlayer1 _returnvalue)
  (bind _returnvalue_2 (Game|SpawnActorfromClass "/Game/HSRFinal/TBPlayer/Player/BP_AOEDPS.BP_AOEDPS_C" (Transformation|GetActorTransform) "Undefined" "MultiplyWithRoot" 0 0))
  (Variables|Default|SetPlayer2 _returnvalue_2)
  (bind _returnvalue_3 (Game|SpawnActorfromClass "/Game/HSRFinal/TBPlayer/Player/BP_Buffer.BP_Buffer_C" (Transformation|GetActorTransform) "Undefined" "MultiplyWithRoot" 0 0))
  (Variables|Default|SetPlayer3 _returnvalue_3)
  (bind _returnvalue_4 (Game|SpawnActorfromClass "/Game/HSRFinal/TBPlayer/Player/BP_Sustain.BP_Sustain_C" (Transformation|GetActorTransform) "Undefined" "MultiplyWithRoot" 0 0))
  (Variables|Default|SetPlayer4 _returnvalue_4)
  ;[0.15 0.15 0.15 0.5] set as hidden
  (for _array_element (Utilities|Array|MakeArray (Variables|Default|GetPlayer1) (Variables|Default|GetPlayer2) (Variables|Default|GetPlayer3) (Variables|Default|GetPlayer4))
    (Rendering|SetActorHiddenInGame _array_element true)))

(fn ConstructionScript)