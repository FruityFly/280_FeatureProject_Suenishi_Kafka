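; BP_STDPS is a player Blueprint in the turn-based player folder, holding only debug logic for its Health attribute.
; Pressing F as a debug key uses the inherited or attached ACAbilitySystem component to apply a large negative Health effect to itself.
; Tick prints the current Health to screen every frame.
; BeginPlay and overlap events are disabled stubs, and the construction script only calls the parent.
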(event EventTick
  (params (DeltaSeconds :type Float%20%28single-precision%29))
  (bind _moddedcurrentvalue (Default|GetAttributeCurrent (Variables|Default|GetAC_AbilitySystem) "Health"))
  (Development|PrintString (Utilities|String|ToString(Float) _moddedcurrentvalue) true true "(R=0.000000,G=0.660000,B=1.000000,A=1.000000)" DeltaSeconds))

(event Collision|EventActorBeginOverlap
  (params (OtherActor :type Actor%20Object%20Reference))
  (|CallParentFunction OtherActor) ; This node is disabled and will not be called.\nDrag off pins to build functionality.
)

(event EventBeginPlay
  (|CallParentFunction) ; This node is disabled and will not be called.\nDrag off pins to build functionality.
)

(event Input|KeyboardEvents|DebugKeyF
  (params (Key :type Key%20Structure :default "None") (ActionValue :type Input%20Action%20Value%20Structure))
  (:Pressed
    (Default|ApplyEffecttoSelf (Variables|Default|GetAC_AbilitySystem) "Health" -1e+03 "NewEnumerator0" "NewEnumerator4" "NewEnumerator0")))

(fn ConstructionScript
  (|CallParentFunction))