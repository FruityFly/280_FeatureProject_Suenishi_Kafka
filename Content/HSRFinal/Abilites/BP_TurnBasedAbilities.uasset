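; Base ability actor for a turn-based combat system, with an empty ActivateAbility event.
; CommitAbility asks the owning ability component whether the ability class can run, then applies a negated cost, currently zero, to a stat as the skill point charge.
; A failed commit destroys the actor and returns false.
; EndAbility fires the CallAbilityEnd dispatcher and destroys the actor, so each ability instance is short-lived.
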(event Custom|ActivateAbility)

(event Custom|EndAbility
  (Default|CallAbilityEnd self)
  (Actor|DestroyActor))

(fn ConstructionScript)

(fn CommitAbility
  ;[0.15 0.15 0.15 0.5] if have enough skill points, commit ability
  (bind _cando (CallFunction|CanDoAbility (Variables|Default|GetOwningAbilityComponent) (Utilities|GetClass self)))
  (if _cando
    (Default|ApplyEffecttoSelf (Variables|Default|GetOwningAbilityComponent) "None" (* (Math|Conversions|ToFloat(Integer) 0) -1.0) "NewEnumerator0" "NewEnumerator4" "NewEnumerator0")
    (return true)
    (else
      (Actor|DestroyActor)
      (return false))))