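; BP_STDPS is a player-side Blueprint under TBPlayer that adds no active logic of its own, leaving behavior to its parent class.
; BeginPlay and overlap events are disabled stubs, Tick is empty, and the construction script only calls the parent.
; Disconnected leftover nodes use ACAbilitySystem to print current Health and apply a large negative Health effect to itself, but never run.
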(event EventTick
  (params (DeltaSeconds :type Float%20%28single-precision%29)))

(event Collision|EventActorBeginOverlap
  (params (OtherActor :type Actor%20Object%20Reference))
  (|CallParentFunction OtherActor) ; This node is disabled and will not be called.\nDrag off pins to build functionality.
)

(event EventBeginPlay
  (|CallParentFunction) ; This node is disabled and will not be called.\nDrag off pins to build functionality.
)

(event Input|KeyboardEvents|DebugKeyF
  (params (Key :type Key%20Structure :default "None") (ActionValue :type Input%20Action%20Value%20Structure)))

(fn ConstructionScript
  (|CallParentFunction))